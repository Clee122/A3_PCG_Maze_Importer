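; Map loader actor that builds a tile grid of water and grass cubes from a text data file on BeginPlay.
; It loads and prints pcg_map_data.txt, then splits the string into rows and reads characters by index.
; A switch on each character spawns BP_WaterCube or BP_GrassCube at a fixed-spacing position, with character index as X and row as Y.
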(event EventBeginPlay
  ;[0 0 0] Read map data in and spawn cube based on position and type
  (bind _loadedstring (Class|DataIOFunctionLibrary|LoadStringfromFile "Data/pcg_map_data.txt"))
  (Development|PrintString _loadedstring)
  ;;[1 1 1] X(rows)
  (for (_array_element _array_index) (Utilities|String|ParseIntoArray _loadedstring " ")
    ;;[1 1 1] Y(volumes)
    (for _index (range (Utilities|String|Len _array_element) 0)
      ;;[1 1 1] Is the character grass? i.e#
      (switch string (Utilities|String|GetSubstring _array_element _index)
        (:Case_0
          ;;[1 1 1] Spawn coloured cube
          (Game|SpawnActorfromClass "/Game/BP_WaterCube.BP_WaterCube_C" (Math|Conversions|ToTransform(Vector) (Math|Vector|MakeVector (Math|Conversions|ToFloat(Integer) (* _index 100)) (Math|Conversions|ToFloat(Integer) (* _array_index 100)) 0.0)) "Undefined" "MultiplyWithRoot" 0 0))
        (:Case_1
          (Game|SpawnActorfromClass "/Game/BP_GrassCube.BP_GrassCube_C" (Math|Conversions|ToTransform(Vector) (Math|Vector|MakeVector (Math|Conversions|ToFloat(Integer) (* _index 100)) (Math|Conversions|ToFloat(Integer) (* _array_index 100)) 0.0)) "Undefined" "MultiplyWithRoot" 0 0))))))

(fn ConstructionScript)
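; Game state for Charles_Game that holds game-wide gravity and move speed values and manages temporary buffs on both.
; Start events clear and restart a five-second timer, so repeat buffs refresh the duration, and reset events restore the default values on expiry.
; RepNotify functions for both values call the gravity and move speed update dispatchers only on the authority.
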(event Custom|StartGravityBuffTimer
  ;[0 0 0] Gravity Buff Timer
  (Utilities|Time|ClearandInvalidateTimerbyHandle (Variables|Default|GetGravityTimerHandle))
  (Development|PrintString "Gravity buff timer refreshed")
  (bind _returnvalue (Utilities|Time|SetTimerbyEvent (EventDispatchers|CreateEvent :!event Custom|ResetGravityBuff) 5.0))
  (Variables|Default|SetGravityTimerHandle _returnvalue))

(event Custom|ResetGravityBuff
  ;[0 0 0] Gravity Buff Timer
  (Variables|Default|SetgameGravity (Variables|Default|GetDefaultGameGravity))
  (Development|PrintString "Gravity buff expired"))

(event Custom|StartMoveSpeedBuffTimer
  ;[0 0 0] MoveSpeed Timer
  (Utilities|Time|ClearandInvalidateTimerbyHandle (Variables|Default|GetMoveSpeedTimerHandle))
  (Development|PrintString "Move speed buff timer refreshed")
  (bind _returnvalue (Utilities|Time|SetTimerbyEvent (EventDispatchers|CreateEvent :!event Custom|ResetMoveSpeedBuff) 5.0))
  (Variables|Default|SetMoveSpeedTimerHandle _returnvalue))

(event Custom|ResetMoveSpeedBuff
  ;[0 0 0] MoveSpeed Timer
  (Variables|Default|SetgameMoveSpeed (Variables|Default|GetDefaultGameMoveSpeed))
  (Development|PrintString "Move speed buff expired"))

(event EventBeginPlay
  (|CallParentFunction) ; This node is disabled and will not be called.\nDrag off pins to build functionality.
)

(event EventTick
  (params (DeltaSeconds :type Float%20%28single-precision%29))
  (|CallParentFunction DeltaSeconds) ; This node is disabled and will not be called.\nDrag off pins to build functionality.
)

(fn ConstructionScript
  (|CallParentFunction))

(fn OnRepGameGravity
  ;[0 0 0] gravity game state
  (Networking|SwitchHasAuthority
    (:Authority
      (Default|CallOnGravityUpdated (Variables|Default|GetgameGravity)))))

(fn OnRepGameMoveSpeed
  ;[0 0 0] move speed game state
  (Networking|SwitchHasAuthority
    (:Authority
      (Default|CallOnMoveSpeedUpdated (Variables|Default|GetgameMoveSpeed)))))
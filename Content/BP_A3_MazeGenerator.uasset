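; Server-side maze generator that, on BeginPlay, spawns a grid of floor tiles with randomly scattered horizontal and vertical walls.
; It first records protected tiles by walking from the grid origin across columns, then randomly stepping rows toward a random far-side goal.
; Protected tiles get debug markers instead of walls, and a corner spawn zone stays clear.
; Path and grid generation both sit inside the entrance-row loop, so they repeat per row.
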(event EventBeginPlay
  (bind _path_tiles (Variables|Default|GetPath%20Tiles))
  ;[0 0 0] spawn walls based on position
  (Networking|SwitchHasAuthority
    (:Authority
      ;;[1 1 1] Create a wide protected entrance zone before random maze generation
      (Utilities|Array|Clear _path_tiles)
      (Variables|Default|SetEntrance%20Start%20Row 1)
      (Variables|Default|SetEntrance%20End%20Row 4)
      (Variables|Default|SetEntrance%20Column 1)
      (for _index (range (Variables|Default|GetEntrance%20Start%20Row) (Variables|Default|GetEntrance%20End%20Row))
        (Utilities|Array|AddUnique _path_tiles (* (Variables|Default|GetGrid%20Width) (Variables|Default|GetEntrance%20Column)))
        ;;[1 1 1] Choose random path start and random goal position
        (Variables|Default|SetPath%20Start%20Row (Math|Random|RandomIntegerinRange (Variables|Default|GetEntrance%20Start%20Row) (Variables|Default|GetEntrance%20End%20Row)))
        (Variables|Default|SetPath%20Start%20Column (Variables|Default|GetEntrance%20Column))
        (Variables|Default|SetGoal%20Row (Math|Random|RandomIntegerinRange 1 (- (Variables|Default|GetGrid%20Height) 2)))
        (Variables|Default|SetGoal%20Column (- (Variables|Default|GetGrid%20Width) 2))
        ;;[1 1 1] Generate protectedpathtiles before spawning maze walls
        (Variables|Default|SetCurrent%20Row 0)
        (Variables|Default|SetCurrent%20Column 0)
        (Utilities|FlowControl|ForLoopwithBreak 0 (+ (Variables|Default|GetGrid%20Width) (Variables|Default|GetGrid%20Height))
          (:LoopBody
            (Utilities|Array|AddUnique _path_tiles (+ (* (Variables|Default|GetCurrent%20Row) (Variables|Default|GetGrid%20Width)) (Variables|Default|GetCurrent%20Column)))
            (if (and (== (Variables|Default|GetCurrent%20Row) (Variables|Default|GetGoal%20Row)) (== (Variables|Default|GetCurrent%20Column) (Variables|Default|GetGoal%20Column)))
              ;;[1 1 1] X(Rows)
              (Utilities|FlowControl|ForLoopwithBreak 0 0)
              (else
                ;;[1 1 1] Update the current path position by moving across column first. Then adjust the rowstowards the goal.
                (if (< (Variables|Default|GetCurrent%20Column) (Variables|Default|GetGoal%20Column))
                  (Variables|Default|SetCurrent%20Column (+ (Variables|Default|GetCurrent%20Column) 1))
                  (elif (Math|Random|RandomBool)
                    (if (< (Variables|Default|GetCurrent%20Row) (Variables|Default|GetGoal%20Row))
                      (Variables|Default|SetCurrent%20Row (+ (Variables|Default|GetCurrent%20Row) 1))
                      (else
                        (Variables|Default|SetCurrent%20Row (- (Variables|Default|GetCurrent%20Row) 1)))))))))
          (:Completed
            (for _index_2 (range 0 (- (Variables|Default|GetGrid%20Height) 1))
              ;;[1 1 1] Y(volumes)
              (for _index_3 (range 0 (- (Variables|Default|GetGrid%20Width) 1))
                ;;[1 1 1] spawn floor
                (Game|SpawnActorfromClass "/Game/BP_Floor.BP_Floor_C" (Math|Conversions|ToTransform(Vector) (Math|Vector|MakeVector (+ (Math|Conversions|ToFloat(Integer) (* _index_3 (Variables|Default|GetTile%20Size))) (Variables|Default|GetMaze%20Offset%20Y)) (+ (Math|Conversions|ToFloat(Integer) (* _index_2 (Variables|Default|GetTile%20Size))) (Variables|Default|GetMaze%20Offset%20X)) 0.0)) "Undefined" "MultiplyWithRoot" 0 0)
                ;;[1 1 1] no walls spawn near player start
                (if (not (and (< _index_2 (Variables|Default|GetSpawn%20Safe%20Size)) (< _index_3 (Variables|Default|GetSpawn%20Safe%20Size))))
                  ;;[1 1 1] Protect entrance and path tiles from random wall spawning.
                  (if (Utilities|Array|ContainsItem (Variables|Default|GetPath%20Tiles) (+ (* _index_2 (Variables|Default|GetGrid%20Width)) _index_3))
                    (Game|SpawnActorfromClass "/Game/BP_A3_PathDebugTile.BP_A3_PathDebugTile_C" (Math|Conversions|ToTransform(Vector) (Math|Vector|MakeVector (+ (Math|Conversions|ToFloat(Integer) (* _index_3 (Variables|Default|GetTile%20Size))) (Variables|Default|GetMaze%20Offset%20Y)) (+ (Math|Conversions|ToFloat(Integer) (* _index_2 (Variables|Default|GetTile%20Size))) (Variables|Default|GetMaze%20Offset%20X)) 0.0)) "Undefined" "MultiplyWithRoot" 0 0)
                    (else
                      ;;[1 1 1] Spawn walls at random position
                      (if (< (Math|Random|RandomIntegerinRange 0 100) 35)
                        (if (Math|Random|RandomBool)
                          (Game|SpawnActorfromClass "/Game/BP_HorizaontalWall.BP_HorizaontalWall_C" (Math|Conversions|ToTransform(Vector) (Math|Vector|MakeVector (+ (Math|Conversions|ToFloat(Integer) (* _index_3 (Variables|Default|GetTile%20Size))) (Variables|Default|GetMaze%20Offset%20Y)) (+ (Math|Conversions|ToFloat(Integer) (* _index_2 (Variables|Default|GetTile%20Size))) (Variables|Default|GetMaze%20Offset%20X)) 0.0)) "Undefined" "MultiplyWithRoot" 0 0)
                          (else
                            (Game|SpawnActorfromClass "/Game/BP_VerticalWall.BP_VerticalWall_C" (Math|Conversions|ToTransform(Vector) (Math|Vector|MakeVector (+ (Math|Conversions|ToFloat(Integer) (* _index_3 (Variables|Default|GetTile%20Size))) (Variables|Default|GetMaze%20Offset%20Y)) (+ (Math|Conversions|ToFloat(Integer) (* _index_2 (Variables|Default|GetTile%20Size))) (Variables|Default|GetMaze%20Offset%20X)) 0.0)) "Undefined" "MultiplyWithRoot" 0 0)))))))))))))))

(fn ConstructionScript)
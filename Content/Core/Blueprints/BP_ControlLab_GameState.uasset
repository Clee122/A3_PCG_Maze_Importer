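; Game state Blueprint for Control Lab that relays replicated match data: remaining time, game over, winner ID, player IDs and experiment state.
; Each RepNotify fires a matching event dispatcher, and the experiment state notify switches between main menu, lobby, playing, paused and game over events.
; Game over is raised by both its own variable and the state switch.
; BeginPlay, Tick and the construction script are empty.
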(event EventBeginPlay)

(event EventTick
  (params (DeltaSeconds :type Float%20%28single-precision%29)))

(fn ConstructionScript)

(fn OnRepRemainingTime
  (Default|CallOnRemainingTimeUpdate (Variables|Default|GetremainingTime)))

(fn OnRepGameOver
  (Default|CallOnGameOver))

(fn OnRepWinnerID
  (Default|CallOnWinnerIDUpdate))

(fn OnRepPlayerIDs
  (Default|CallOnPlayerIDUpdate))

(fn OnRepExperimentState
  (switch Utilities|FlowControl|Switch|SwitchonEControlLab_ExperimentState (Variables|Default|GetexperimentState)
    (:NewEnumerator0
      (Default|CallOnMainMenu))
    (:NewEnumerator1
      (Default|CallOnLobby))
    (:NewEnumerator2
      (Default|CallOnGamePlaying))
    (:NewEnumerator3
      (Default|CallOnGamePaused))
    (:NewEnumerator4
      (Default|CallOnGameOver))))
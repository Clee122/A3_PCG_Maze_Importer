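; BP_ControlLab_GameMode is the game mode for the Control Lab, handling manager startup and player registration.
; On BeginPlay, the authority spawns a BP_ControllLab_Manager at the world origin.
; On PostLogin, it adds the new player's PlayerId uniquely to the PlayerIDs array on BP_ControlLab_GameState, then calls CallOnPlayerIDUpdate to signal the change.
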(event EventBeginPlay
  ;[0 0 0] Spawn control lab manager if server
  (Networking|SwitchHasAuthority
    (:Authority
      (Game|SpawnActorfromClass "/Game/Core/Blueprints/BP_ControllLab_Manager.BP_ControllLab_Manager_C" (Math|Transform|MakeTransform "0, 0, 0") "Undefined" "MultiplyWithRoot" 0 0))))

(event EventPostLogin
  (params (NewPlayer :type Player%20Controller%20Object%20Reference))
  ;[0 0 0] Join Game - Point login
  (bind _asbp_control_lab_game_state (Utilities|Casting|CastToBP_ControlLab_GameState (Game|GetGameState)))
  (Utilities|Array|AddUnique (Variables|/Game/Core/Blueprints/BP_ControlLab_GameState.BP_ControlLab_GameState_C|GetPlayerIDs _asbp_control_lab_game_state) (Variables|/Script/Engine.PlayerState|GetPlayerId (Variables|/Script/Engine.Controller|GetPlayerState NewPlayer)))
  (Default|CallOnPlayerIDUpdate _asbp_control_lab_game_state))

(fn ConstructionScript)
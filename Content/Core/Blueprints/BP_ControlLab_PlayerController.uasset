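; Player controller for ControlLab that switches UI, input mode and cursor as the game moves between lobby, playing and game over.
; On BeginPlay it binds to BP_ControlLab_GameState events and triggers the lobby; locally, lobby shows a menu widget and playing swaps it for a timer HUD.
; Escape (or 1 for editor debugging) exits: the server travels to the main menu, clients disconnect, and both destroy the session and remove a player ID.
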(event Custom|OnGameOver
  ;[0 0 0] Game Over
  (Input|SetIgnoreMoveInput true)
  (Input|SetIgnoreLookInput true)
  (Input|SetInputModeUIOnly self 0 "DoNotLock" false)
  (Variables|Default|SetbShowMouseCursor true))

(event Custom|OnExitGame
  ;[0 0 0] Exit Game
  ;;[1 1 1] Are we the server?
  (if (Networking|IsServer)
    ;;[1 1 1] Exit as server and kick other players.
    (Development|ExecuteConsoleCommand (Utilities|String|Append "ServerTravel " (Variables|Default|GetMainMenuName)) 0)
    (|DestroySession (Game|GetPlayerController 0)
      (:then
        _))
    (else
      ;;[1 1 1] Exit session as player
      (|DestroySession (Game|GetPlayerController 0)
        (:then
          (Development|ExecuteConsoleCommand "disconnect" (Game|GetPlayerController 0))))))
  ;;[1 1 1] Remove player id
  (bind _asbp_control_lab_game_state (Utilities|Casting|CastToBP_ControlLab_GameState (Game|GetGameState)))
  (Utilities|Array|RemoveItem (Variables|/Game/Core/Blueprints/BP_ControlLab_GameState.BP_ControlLab_GameState_C|GetplayerIDs _asbp_control_lab_game_state) (Variables|/Script/Engine.PlayerState|GetPlayerId (Game|GetPlayerState 0))))

(event Custom|OnGamePlaying
  ;[0 0 0] Game Playing
  (if (Pawn|IsLocalController)
    (Class|Controller|ResetIgnoreInputFlags)
    (Input|SetIgnoreMoveInput false)
    (Input|SetIgnoreLookInput false)
    (Viewport|RemoveAllWidgets)
    (CallFunction|AddHUDTimer)
    (Input|SetInputModeGameOnly self false)
    (Variables|Default|SetbShowMouseCursor false)))

(event Custom|OnGameLobby
  ;[0 0 0] Game Lobby
  (if (Pawn|IsLocalController)
    (Input|SetIgnoreMoveInput true)
    (Input|SetIgnoreLookInput true)
    (bind _returnvalue (UserInterface|CreateWidget "/Game/Core/UI/WBP_GameLobby.WBP_GameLobby_C"))
    (bind _output_get (Variables|Default|SetLobbyWidgetRef _returnvalue))
    (Input|SetInputModeUIOnly self _output_get "DoNotLock" false)
    (Variables|Default|SetbShowMouseCursor true)
    (UserInterface|Viewport|AddtoViewport _output_get 0)))

(event EventBeginPlay
  ;[0 0 0] OnBeginPlay Switch to player controller input, from UI input
  (bind _asbp_control_lab_game_state (Utilities|Casting|CastToBP_ControlLab_GameState (Game|GetGameState)))
  (Variables|Default|SetControlLabGameStateRef _asbp_control_lab_game_state)
  (EventDispatchers|BindEventtoOnGameOver (Variables|Default|GetControlLabGameStateRef) (EventDispatchers|CreateEvent :!event Custom|OnGameOver))
  (EventDispatchers|BindEventtoOnGamePlaying (Variables|Default|GetControlLabGameStateRef) (EventDispatchers|CreateEvent :!event Custom|OnGamePlaying))
  (EventDispatchers|BindEventtoOnLobby (Variables|Default|GetControlLabGameStateRef) (EventDispatchers|CreateEvent :!event Custom|OnGameLobby))
  (Default|CallOnLobby (Variables|Default|GetControlLabGameStateRef)))

(event Input|KeyboardEvents|Escape
  (params (Key :type Key%20Structure :default "None"))
  ;[0 0 0] On Press "ESC" to exit. TODO: implement pause screen ;)
  (:Pressed
    (CallFunction|OnExitGame)))

(event Input|KeyboardEvents|1
  (params (Key :type Key%20Structure :default "None"))
  ;[0 0 0] On Press "ESC" to exit. TODO: implement pause screen ;)
  ;;[1 1 1] Used for debugging as "esc" key closes the editor runtime
  (:Pressed
    (CallFunction|OnExitGame)))

(fn ConstructionScript)

(fn DisablePlayerInput
  (Input|SetIgnoreMoveInput true)
  (Input|SetIgnoreLookInput true)
  (Input|SetInputModeUIOnly 0 0 "DoNotLock" false)
  (Variables|Default|SetbShowMouseCursor true))

(fn AddHUDTimer
  (bind _returnvalue (UserInterface|CreateWidget "/Game/Core/UI/WBP_HUD_TIMER.WBP_HUD_TIMER_C"))
  (bind _output_get (Variables|Default|SetTimerWidgetRef _returnvalue))
  (bind _output_get_2 (Variables|Default|SetTimerHudReference _output_get))
  (UserInterface|Viewport|AddtoViewport _output_get_2 0)
  (Input|SetInputModeGameOnly (Game|GetPlayerController 0) false))

(fn OnRepLobbyWidgetRef)

(fn OnRepTimerWidgetRef)

(fn OnRepTimerHudReference)
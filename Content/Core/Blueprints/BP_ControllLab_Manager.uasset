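; Server-side round manager for the ControlLab experiment, handling the countdown and round end.
; On BeginPlay the authority puts BP_ControlLab_GameState into lobby state and starts a one-second timer that decrements RemainingTime only while playing.
; Timeout calls EndRound with winner -1.
; EndRound records the winner, sets GameOver once, then after a short delay resets by ServerTravel to the PCG maze map.
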(event Custom|UpdateTimer
  ;[0 0 0] Update Game Timer
  (switch Utilities|FlowControl|Switch|SwitchonEControlLab_ExperimentState (Variables|/Game/Core/Blueprints/BP_ControlLab_GameState.BP_ControlLab_GameState_C|GetexperimentState (Variables|Default|GetControlLabGameStateRef))
    (:NewEnumerator2
      ;;[1 1 1] Update Timer
      (bind _output_get (Variables|/Game/Core/Blueprints/BP_ControlLab_GameState.BP_ControlLab_GameState_C|SetremainingTime (Variables|Default|GetControlLabGameStateRef) (- (Variables|/Game/Core/Blueprints/BP_ControlLab_GameState.BP_ControlLab_GameState_C|GetremainingTime (Variables|Default|GetControlLabGameStateRef)) 1.0)))
      ;;[1 1 1] If Timer runs out. Game Over
      (if (<= _output_get 0.0)
        (CallFunction|EndRound -1)))))

(event Custom|EndRound
  (params (WinnerID :type Integer))
  (bind _controllabgamestateref (Variables|Default|GetControlLabGameStateRef))
  ;[0 0 0] reset after a round
  (Development|PrintString "\"EndRound started\"")
  (Networking|SwitchHasAuthority
    (:Authority
      (Development|PrintString "\"Authority passed\"")
      (if (not (Utilities|Enum|Equal(Enum) (Variables|/Game/Core/Blueprints/BP_ControlLab_GameState.BP_ControlLab_GameState_C|GetexperimentState _controllabgamestateref) "NewEnumerator4"))
        (Development|PrintString "\"Setting result\"")
        (Variables|/Game/Core/Blueprints/BP_ControlLab_GameState.BP_ControlLab_GameState_C|SetwinnerID _controllabgamestateref WinnerID)
        (Variables|/Game/Core/Blueprints/BP_ControlLab_GameState.BP_ControlLab_GameState_C|SetexperimentState _controllabgamestateref "NewEnumerator4")
        (Development|PrintString "Game over!")
        (Utilities|Time|ClearandInvalidateTimerbyHandle (Variables|Default|GetTimerHandle_Experiment))
        (Development|PrintString "\"Before reset delay\"")
        (Utilities|FlowControl|Delay 2.0)
        (Development|PrintString "\"After reset delay\"")
        (Development|ExecuteConsoleCommand "ServerTravel /Game/Experiments/Charles_Game/A3_PCG_Maze_Importer?listen" 0)))))

(event EventBeginPlay
  (Networking|SwitchHasAuthority
    (:Authority
      (bind _asbp_control_lab_game_state (Utilities|Casting|CastToBP_ControlLab_GameState (Game|GetGameState)))
      (Variables|Default|SetControlLabGameStateRef _asbp_control_lab_game_state)
      (Variables|/Game/Core/Blueprints/BP_ControlLab_GameState.BP_ControlLab_GameState_C|SetremainingTime (Variables|Default|GetControlLabGameStateRef) (Variables|/Game/Core/Blueprints/BP_ControlLab_GameState.BP_ControlLab_GameState_C|GetremainingTime (Variables|Default|GetControlLabGameStateRef)))
      (Variables|/Game/Core/Blueprints/BP_ControlLab_GameState.BP_ControlLab_GameState_C|SetexperimentState (Variables|Default|GetControlLabGameStateRef) "NewEnumerator1")
      (Utilities|Time|SetTimerbyEvent (delegate Custom|UpdateTimer) 1.0 true))))

(fn ConstructionScript)

(fn OnRepRemainingTime
  (Development|PrintString "RemainingTime"))